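; BP_Laser is an effect actor that displays a red Niagara laser beam along its forward direction.
; BeginPlay sets the beam color on the Niagara component.
; Each tick it line traces on the Visibility channel up to a fixed range and feeds the hit point, or the maximum range point, into the LaserEnd parameter.
; The trace also draws a one-frame debug line, and hits only shorten the beam visually.
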(event EventTick
  (params (DeltaSeconds :type Float%20%28single-precision%29))
  (bind _returnvalue (Transformation|GetActorForwardVector))
  (bind _returnvalue_2 (Transformation|GetActorLocation))
  (bind _returnvalue_3 (* _returnvalue 1.5e+03))
  (bind _returnvalue_4 (+ _returnvalue_2 _returnvalue_3))
  (bind (_outhit _returnvalue_5) (Collision|LineTraceByChannel _returnvalue_2 _returnvalue_4 "TraceTypeQuery1" false 0 "ForOneFrame"))
  (Effects|Components|ParticleSystem|SetVectorParameter (Variables|Default|GetNiagaraLaser) "LaserEnd" (select _returnvalue_5 (.location _outhit) _returnvalue_4)))

(event EventBeginPlay
  (Effects|Components|ParticleSystem|SetColorParameter (Variables|Default|GetNiagaraLaser) "BeamColor" "(R=1.000000,G=0.000000,B=0.007180,A=1.000000)"))

(fn ConstructionScript)