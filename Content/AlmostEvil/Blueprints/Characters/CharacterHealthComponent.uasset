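; Health component for characters that tracks health, applies damage and healing, and signals death.
; On BeginPlay it fills Health to MaxHealth and binds to its owner's OnTakeAnyDamage event.
; Damage applies only while health is positive and calls DeathMessage on the owner at zero or below, while healing clamps to the maximum.
; Health's RepNotify broadcasts changes through the OnHealthChanged dispatcher.
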(event Custom|OnTakeAnyDamage
  (params (DamagedActor :type Actor%20Object%20Reference) (Damage :type Float%20%28single-precision%29) (DamageType :type Damage%20Type%20Object%20Reference) (InstigatedBy :type Controller%20Object%20Reference) (DamageCauser :type Actor%20Object%20Reference))
  (if (> (Variables|Default|GetHealth) 0.0)
    (Variables|Default|SetHealth (- (Variables|Default|GetHealth) Damage))
    (if (<= (Variables|Default|GetHealth) 0.0)
      (Class|IDamageable|Death(Message) (Components|GetOwner)))))

(event Custom|Heal
  (params (Amount :type Float%20%28single-precision%29))
  (Variables|Default|SetHealth (Math|Float|Clamp(Float) (+ Amount (Variables|Default|GetHealth)) 0.0 (Variables|Default|GetMaxHealth))))

(event EventBeginPlay
  (Variables|Default|SetHealth (Variables|Default|GetMaxHealth))
  (EventDispatchers|AssignOnTakeAnyDamage (Components|GetOwner) (delegate Custom|OnTakeAnyDamage)))

(fn OnRepHealth
  (Default|CallOnHealthChanged (Variables|Default|GetHealth)))