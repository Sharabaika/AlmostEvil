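; Grenade launcher projectile that explodes when its projectile movement component stops.
; On impact it draws a debug sphere and spawns an explosion emitter and sound at the hit location.
; Only the authority applies radial damage credited to the instigator, hides the box component, reports an AI noise event, and destroys the actor after a short delay.
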(event OnProjectileStop(ProjectileMovementComponent)
  (params (ImpactResult :type Hit%20Result%20Structure%20%28by%20ref%29))
  (Rendering|Debug|DrawDebugSphere (.location ImpactResult) 1e+02 12 "(R=1.000000,G=1.000000,B=1.000000,A=1.000000)" 1.0)
  (Networking|SwitchHasAuthority
    (:Authority
      (Game|Damage|ApplyRadialDamage (Variables|Default|GetMaxDamage) (.location ImpactResult) (Variables|Default|GetMaxRange) 0 0 self (Game|GetInstigatorController) false "ECC_Visibility")
      (Rendering|SetVisibility (Variables|Default|GetBoxComponent) false false)
      (Class|AISenseHearing|ReportNoiseEvent (Transformation|GetActorLocation) 1.0 0 0.0 "Noise")
      (Utilities|FlowControl|Delay 0.2) ; kek
      (Actor|DestroyActor))
    (:Remote
      _))
  (Effects|SpawnEmitteratLocation "/Game/Models/Weapons/MilitaryWeapDark/FX/P_RocketLauncher_Explosion_01.P_RocketLauncher_Explosion_01" (.location ImpactResult))
  (Audio|SpawnSoundatLocation "/Game/Models/Weapons/MilitaryWeapDark/Sound/GrenadeLauncher/Wavs/GrenadeLauncher_Explosion02.GrenadeLauncher_Explosion02" (.location ImpactResult) "0, 0, 0" 1.0 1.0 0.0 0 0))

(fn ConstructionScript)