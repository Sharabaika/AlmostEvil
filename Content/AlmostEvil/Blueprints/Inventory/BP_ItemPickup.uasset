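; BP_ItemPickup is an interactable world pickup for an inventory item.
; Its construction script enables box physics, looks up the item's row in DT_Items to store the data and set the mesh, and destroys the actor if no row is found.
; Interacting passes the pickup to the third-person character's InventoryComponent.
; DestroyIfEmpty removes it at zero quantity, and a rotator component targets the mesh from BeginPlay.
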(event Custom|DestroyIfEmpty
  (if (not (Math|Conversions|ToBoolean(Integer) (Variables|Default|GetQuantity)))
    (Actor|DestroyActor)))

(event EventInteract
  (params (Interactor :type Third%20Person%20Character%20Object%20Reference))
  (bind _asbp_third_person_character (Utilities|Casting|CastToBP_ThirdPersonCharacter Interactor))
  (Default|PickUpItems (Variables|/Game/AlmostEvil/Blueprints/Characters/BP_ThirdPersonCharacter.BP_ThirdPersonCharacter_C|GetInventoryComponent _asbp_third_person_character) self))

(event EventBeginPlay
  (Variables|/Script/AlmostEvil.ComponentRotator|SetComponentToRotate (Variables|Default|GetComponentRotator) (Variables|Default|GetStaticMesh)))

(fn ConstructionScript
  (Physics|SetSimulatePhysics (Variables|Default|GetBoxComponent) true)
  (bind _returnvalue (Utilities|GetDataTableRow "/Game/AlmostEvil/Blueprints/Inventory/DT_Items.DT_Items" (.rowname (Variables|Default|GetItem)))
    (:then
      (CallFunction|SetupPickupData _returnvalue))
    (:RowNotFound
      (Actor|DestroyActor))))

(fn GetIsActive
  (return true))

(fn UsebyCharacter
  (params (Character :type BP%20Third%20Person%20Character%20Object%20Reference)))

(fn SetupPickupData
  (params (ItemData :type S%20Item%20Data%20Structure))
  (bind _output_get (Variables|Default|SetItemData ItemData))
  (Utilities|IsValid (.mesh _output_get)
    (:Is%20Valid
      (Components|StaticMesh|SetStaticMesh (Variables|Default|GetStaticMesh) (.mesh _output_get)))))