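; BP_StateTrigger is a trigger volume that changes the level state of the co-op game when a player enters it.
; On Box overlap, it casts the other actor to BP_ThirdPersonCharacter and runs CheckRequirements, which passes only for player-controlled characters.
; UpdateLevelState then hands NewLevelState to BP_CoopGameState.
; Nothing here disables the trigger, so each qualifying overlap sends the state again.
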(event OnComponentBeginOverlap(Box)
  (params (OverlappedComponent :type Primitive%20Component%20Object%20Reference) (OtherActor :type Actor%20Object%20Reference) (OtherComp :type Primitive%20Component%20Object%20Reference) (OtherBodyIndex :type Integer) (bFromSweep :type Boolean) (SweepResult :type Hit%20Result%20Structure%20%28by%20ref%29))
  (bind _asbp_third_person_character (Utilities|Casting|CastToBP_ThirdPersonCharacter OtherActor))
  (bind _canupdatestate (CallFunction|CheckRequirements _asbp_third_person_character))
  (if _canupdatestate
    (CallFunction|UpdateLevelState)))

(fn ConstructionScript)

(fn UpdateLevelState
  (bind _asbp_coop_game_state (Utilities|Casting|CastToBP_CoopGameState (Game|GetGameState)))
  (Default|UpdateLevelState _asbp_coop_game_state (Variables|Default|GetNewLevelState)))

(fn CheckRequirements
  (params (TriggeredCharacter :type BP%20Third%20Person%20Character%20Object%20Reference))
  (return (Pawn|IsPlayerControlled TriggeredCharacter)))