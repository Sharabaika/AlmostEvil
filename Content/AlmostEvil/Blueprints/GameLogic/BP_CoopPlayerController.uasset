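; Player controller for a co-op game that handles character switching, inventory and pause menu input, and leaving the session for the main menu.
; Switch requests go to BP_CoopGameMode, while the inventory toggle locks look input, shows a centered cursor, disables aiming and fires OnInventoryInput.
; Possess and UnPossess recolor the character from the cached BP_CoopPlayerState and both call OnPossessedClient, which runs the character's OnPossessedSafe.
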(event Custom|TrySwitchCharacter
  ;[1 1 1] Possessing
  (bind _asbp_coop_game_mode (Utilities|Casting|CastToBP_CoopGameMode (Game|GetGameMode)))
  (Default|TrySwitchActiveCharacterforPlayer _asbp_coop_game_mode self))

(event Custom|OnPossessed_Client
  (params (Possessed%20Pawn :type Pawn%20Object%20Reference))
  ;[1 1 1] Possessing
  (bind _asbp_third_person_character (Utilities|Casting|CastToBP_ThirdPersonCharacter Possessed%20Pawn))
  (Default|OnPossessedSafe _asbp_third_person_character))

(event Custom|ExitToMainMenu
  (Utilities|FlowControl|Sequence
    (:then_0
      (|DestroySession self))
    (:then_1
      (Game|OpenLevel(byName) "MainMenu"))))

(event EventPossess
  (params (PossessedPawn :type Pawn%20Object%20Reference))
  (bind _coopplayerstate (Variables|Default|GetCoopPlayerState))
  ;[1 1 1] Possessing
  (CallFunction|OnPossessedClient PossessedPawn)
  ;;[1 1 1] Setting character's color
  (bind _asbp_third_person_character (Utilities|Casting|CastToBP_ThirdPersonCharacter PossessedPawn))
  (Utilities|IsValid _coopplayerstate
    (:Is%20Valid
      (Variables|/Game/AlmostEvil/Blueprints/Characters/BP_ThirdPersonCharacter.BP_ThirdPersonCharacter_C|SetCharacterColor _asbp_third_person_character (Variables|/Game/AlmostEvil/Blueprints/GameLogic/BP_CoopPlayerState.BP_CoopPlayerState_C|GetPlayerColor _coopplayerstate)))))

(event EventUnPossess
  (params (UnpossessedPawn :type Pawn%20Object%20Reference))
  (bind _coopplayerstate (Variables|Default|GetCoopPlayerState))
  ;[1 1 1] Possessing
  (CallFunction|OnPossessedClient UnpossessedPawn)
  ;;[1 1 1] Setting character's color
  (bind _asbp_third_person_character (Utilities|Casting|CastToBP_ThirdPersonCharacter UnpossessedPawn))
  (Utilities|IsValid _coopplayerstate
    (:Is%20Valid
      (Variables|/Game/AlmostEvil/Blueprints/Characters/BP_ThirdPersonCharacter.BP_ThirdPersonCharacter_C|SetCharacterColor _asbp_third_person_character (Variables|/Game/AlmostEvil/Blueprints/GameLogic/BP_CoopPlayerState.BP_CoopPlayerState_C|GetDefaultPlayerColor _coopplayerstate)))))

(event EventBeginPlay
  (bind _self self)
  (Input|EnableInput _self)
  (Input|SetInputModeGameandUI _self 0 "LockAlways" true)
  (bind _asbp_coop_player_state (Utilities|Casting|CastToBP_CoopPlayerState (Variables|GetPlayerState)))
  (Variables|Default|SetCoopPlayerState _asbp_coop_player_state))

(event Input|ActionEvents|InputActionSwitchCharacter
  (params (Key :type Key%20Structure))
  ;[1 1 1] Possessing
  (:Pressed
    (CallFunction|TrySwitchCharacter)))

(event Input|ActionEvents|InputActionOpenInventory
  (params (Key :type Key%20Structure))
  (bind (_sizex _sizey) (HUD|GetViewportSize))
  ;[1 1 1] Input
  (:Pressed
    (bind _output_get (Variables|Default|SetisInInventory (not (Variables|Default|GetisInInventory))))
    (Input|SetIgnoreLookInput _output_get)
    (Class|PlayerController|SetMouseLocation (/ _sizex 2) (/ _sizey 2))
    (Variables|Default|SetbShowMouseCursor _output_get)
    (Default|CallOnInventoryInput _output_get)
    (bind _asbp_third_person_character (Utilities|Casting|CastToBP_ThirdPersonCharacter (Pawn|GetControlledPawn)))
    (Variables|/Script/AlmostEvil.ThirdPersonCharacter|SetCanAim _asbp_third_person_character (not _output_get))
    (Class|ThirdPersonCharacter|StopAimInput _asbp_third_person_character)))

(event Input|ActionEvents|InputActionOpenPauseMenu
  (params (Key :type Key%20Structure))
  ;[1 1 1] Input
  (:Pressed
    (bind _asplayer_hud (Utilities|Casting|CastToPlayerHUD (HUD|GetHUD)))
    (Default|ShowPauseMenu _asplayer_hud true)))

(fn ConstructionScript)