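; BP_DetonateOnDamage is a map object that explodes when it takes damage above a threshold.
; Any damage or radial damage over that threshold calls Detonate, which disables further damage and waits on a timer.
; It then spawns explosion particles and sound, applies radial damage around itself and destroys the actor.
; Because the blast is radial damage, it can set off other such objects nearby.
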(event Custom|Detonate
  (Variables|Actor|SetbCanBeDamaged false)
  (Utilities|FlowControl|Delay (Variables|Default|GetDetonationTimer))
  (CallFunction|DetonationEffects)
  (Game|Damage|ApplyRadialDamage (Variables|Default|GetDetonationDamage) (Transformation|GetActorLocation) (Variables|Default|GetDetonationRadius) 0 (Utilities|Array|MakeArray self) 0 0 false "ECC_Visibility")
  (Actor|DestroyActor))

(event Custom|DetonationEffects
  (Effects|SpawnEmitteratLocation (Variables|Default|GetExplosion) (Transformation|GetActorLocation))
  (Audio|SpawnSoundatLocation (Variables|Default|GetExplostionSound) (Transformation|GetActorLocation) "0, 0, 0" 1.0 1.0 0.0 0 0))

(event Game|Damage|EventRadialDamage
  (params (DamageReceived :type Float%20%28single-precision%29) (DamageType :type Damage%20Type%20Object%20Reference) (Origin :type Vector :default "0, 0, 0") (HitInfo :type Hit%20Result%20Structure%20%28by%20ref%29) (InstigatedBy :type Controller%20Object%20Reference) (DamageCauser :type Actor%20Object%20Reference))
  (if (> DamageReceived (Variables|Default|GetDetonationDamageTreshold))
    (CallFunction|Detonate)))

(event Game|Damage|EventAnyDamage
  (params (Damage :type Float%20%28single-precision%29) (DamageType :type Damage%20Type%20Object%20Reference) (InstigatedBy :type Controller%20Object%20Reference) (DamageCauser :type Actor%20Object%20Reference))
  (if (> Damage (Variables|Default|GetDetonationDamageTreshold))
    (CallFunction|Detonate)))

(fn ConstructionScript)