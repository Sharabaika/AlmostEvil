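; Game instance that manages multiplayer sessions, server level travel and the loading screen for the game's menus.
; It hosts an advanced session with LAN option and custom server name, opening Lobby as a listen server, and joins sessions from search results or accepted invites.
; ServerTravel console commands load the lobby or levels, storing the current level for reloads.
; Network and travel error handlers are empty.
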(event Custom|LoadLevel
  (params (Level :type Level%20Selection%20Struct%20Structure))
  (Variables|Default|SetCurrentLevel Level)
  (Variables|Default|SetCurrentLevelIsSet true)
  (Development|ExecuteConsoleCommand (Utilities|String|Append "ServerTravel " (.LevelFileName (Utilities|Struct|BreakLevelSelectionStruct Level))) (Game|GetPlayerController 0)))

(event Custom|ReloadCurrentLevel
  (if (Variables|Default|GetCurrentLevelIsSet)
    (CallFunction|LoadLevel (Variables|Default|GetCurrentLevel))))

(event Custom|JoinServer
  (params (Session :type Blueprint%20Session%20Result%20Structure))
  (CallFunction|ShowLoadingScreen)
  (|JoinSession (Game|GetPlayerController 0) Session))

(event Custom|LoadLobbyMenu
  (Development|ExecuteConsoleCommand (Utilities|String|Append "ServerTravel " "Lobby") (Game|GetPlayerController 0)))

(event Custom|HideActiveMenu
  (bind _activemenu (Variables|Menus|GetActiveMenu)
    (:then
      (Widget|RemovefromParent _activemenu))
    (:else)))

(event Custom|LaunchLobby
  (params (EnableLan :type Boolean) (ServerName :type String) (MaxPlayers :type Integer))
  (CallFunction|ShowLoadingScreen)
  (|AdvancedSession (Utilities|Array|MakeArray (Class|AdvancedSessionsLibrary|MakeLiteralSessionPropertyString "ServerName" ServerName)) (Game|GetPlayerController 0) MaxPlayers 0 EnableLan true false true true false false false true
    (:OnSuccess
      (Game|OpenLevel(byName) "Lobby" true "listen"))))

(event Custom|ShowLoadingScreen
  (CallFunction|HideActiveMenu)
  (Variables|Menus|GetLoadingScreen
    (:then
      _)
    (:else
      (bind _returnvalue (UserInterface|CreateWidget "/Game/AlmostEvil/Blueprints/Menuing/MainMenu/Widgets/W_LoadingScreen.W_LoadingScreen_C" (Game|GetPlayerController 0)))
      (bind _output_get (Variables|Menus|SetLoadingScreen _returnvalue))))
  (UserInterface|Viewport|AddtoViewport _output_get 0)
  (Variables|Menus|SetActiveMenu _output_get))

(event Custom|DestroySessionCaller
  (params (Caller :type Player%20Controller%20Object%20Reference))
  (|DestroySession Caller))

(event EventHandleNetworkError
  (params (FailureType :type ENetworkFailure%20Enum :default "NetDriverAlreadyExists") (bIsServer :type Boolean)))

(event EventHandleTravelError
  (params (FailureType :type ETravelFailure%20Enum :default "NoLevel")))

(event EventOnSessionInviteAccepted
  (params (LocalPlayerNum :type Integer) (PersonInvited :type BP%20Unique%20Net%20Id%20Structure) (SessionToJoin :type Blueprint%20Session%20Result%20Structure%20%28by%20ref%29))
  (|JoinSession 0 SessionToJoin))