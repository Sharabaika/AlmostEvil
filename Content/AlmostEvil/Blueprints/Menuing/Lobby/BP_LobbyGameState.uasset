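; BP_LobbyGameState is the lobby's game state, tracking the joined players and the selected level.
; Players and CurrentLevelIndex use RepNotify to fire update dispatchers, which AddPlayer and SelectLevel also call directly after changing them.
; GetCanStartGame returns true only when every listed player is either the host or ready.
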(event Custom|AddPlayer
  (params (Player :type BP%20Lobby%20Player%20State%20Object%20Reference%20%28by%20ref%29))
  (Utilities|Array|AddUnique (Variables|Default|GetPlayers) Player)
  (CallFunction|CallUpdatePlayers))

(fn ConstructionScript)

(fn OnRepPlayers
  (Default|CallOnPlayersUpdated (Variables|Default|GetPlayers)))

(fn CallUpdatePlayers
  (Default|CallOnPlayersUpdated (Variables|Default|GetPlayers)))

(fn GetCanStartGame
  (for _array_element (Variables|Default|GetPlayers)
    (if (not (or (Variables|/Game/AlmostEvil/Blueprints/Menuing/Lobby/BP_LobbyPlayerState.BP_LobbyPlayerState_C|GetisHost _array_element) (Variables|/Game/AlmostEvil/Blueprints/Menuing/Lobby/BP_LobbyPlayerState.BP_LobbyPlayerState_C|GetisReady _array_element)))
      (return false)))
  (return true))

(fn OnRepCurrentLevelIndex
  (Default|CallOnCurrentLevelIndexSet (Variables|Default|GetCurrentLevelIndex)))

(fn SelectLevel
  (params (CurrentLevelIndex :type Integer))
  (bind _output_get (Variables|Default|SetCurrentLevelIndex CurrentLevelIndex))
  (Default|CallOnCurrentLevelIndexSet _output_get))