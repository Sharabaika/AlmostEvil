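; AI controller for zombie enemies that runs BT_Zombie and turns perception updates into blackboard state.
; Sighted actors become the focus and attack target, preferring the nearer one; lost sight switches to another visible actor or searches the last location.
; Noise starts a search only when no target is held.
; Attack, search and stroll helpers set AI state, focus and the pawn's running flag, while TryToAttack triggers the pawn's attack.
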(event OnTargetPerceptionUpdated(AIPerception)
  (params (Actor :type Actor%20Object%20Reference) (Stimulus :type AI%20Stimulus%20Structure))
  (CallFunction|OnPreceptionUpdated Actor Stimulus))

(event Custom|TryToAttack
  (bind _asbp_enemy_base (Utilities|Casting|CastToBP_EnemyBase (Pawn|GetControlledPawn)))
  (Default|StartAttack _asbp_enemy_base true))

(event EventBeginPlay
  (AI|RunBehaviorTree "/Game/AlmostEvil/Blueprints/Characters/Enemies/AI/BT_Zombie.BT_Zombie"))

(fn ConstructionScript)

(fn OnPreceptionUpdated
  (params (Actor :type Actor%20Object%20Reference) (AIStimulus :type AI%20Stimulus%20Structure%20%28by%20ref%29))
  (bind (_age _expirationage _strength _stimuluslocation _receiverlocation _tag _bsuccessfullysensed) (Utilities|Struct|BreakAIStimulus AIStimulus))
  (bind _returnvalue (Class|AIController|GetFocusActor))
  (bind _aiperception (Variables|Default|GetAIPerception))
  (bind _outactors (Class|AIPerceptionComponent|GetPerceivedActors _aiperception "/Script/AIModule.AISense_Sight"))
  (switch name _tag
    (:Default
      (if _bsuccessfullysensed ; if gets  new target
        ;[1 1 1] if already has target
        (Utilities|IsValid _returnvalue ; IfHasTargetActor
          (:Is%20Valid
            (bind _besttarget (CallFunction|ChooseBestTarget _returnvalue Actor))
            (CallFunction|AttackTarget _besttarget))
          (:Is%20Not%20Valid
            (CallFunction|AttackTarget Actor)))
        (elif (Math|Conversions|ToBoolean(Integer) (Utilities|Array|Length _outactors)) ; if has any other targets
          ;[1 1 1] choose any other visible target
          (CallFunction|AttackTarget (Utilities|Array|Get(acopy) _outactors))
          (else
            ;[1 1 1] search for the lost target
            (CallFunction|StartSearching (Transformation|GetActorLocation Actor))))))
    (:Noise
      (if _bsuccessfullysensed
        (Utilities|IsValid (Class|AIController|GetFocusActor) ; if does not have target
          (:Is%20Not%20Valid
            (CallFunction|StartSearching (.stimuluslocation AIStimulus))))))))

(fn ChooseBestTarget
  (params (First :type Actor%20Object%20Reference) (Second :type Actor%20Object%20Reference))
  (bind _returnvalue (Pawn|GetControlledPawn))
  (bind _returnvalue_2 (Transformation|GetActorLocation _returnvalue))
  (return (select (< (Class|KismetMathLibrary|VectorDistanceSquared (Transformation|GetActorLocation First) _returnvalue_2) (Class|KismetMathLibrary|VectorDistanceSquared _returnvalue_2 (Transformation|GetActorLocation Second))) First Second)))

(fn AttackTarget
  (params (Target :type Actor%20Object%20Reference))
  (bind _blackboard (Variables|Default|GetBlackboard))
  (AI|Components|Blackboard|SetValueasObject _blackboard (Utilities|Name|MakeLiteralName "TargetActror") Target)
  (AI|Components|Blackboard|SetValueasEnum _blackboard (Utilities|Name|MakeLiteralName "AIState") (Utilities|Enum|LiteralenumBPE_EnamyAIState "NewEnumerator2"))
  (AI|SetFocus Target)
  (bind _asbp_enemy_base (Utilities|Casting|CastToBP_EnemyBase (Pawn|GetControlledPawn)))
  (Default|SetIsRunning _asbp_enemy_base true))

(fn StartSearching
  (params (AtLocation :type Vector))
  (bind _blackboard (Variables|Default|GetBlackboard))
  (AI|Components|Blackboard|SetValueasVector _blackboard (Utilities|Name|MakeLiteralName "LastSeenTargetLocation") AtLocation)
  (AI|Components|Blackboard|SetValueasEnum _blackboard (Utilities|Name|MakeLiteralName "AIState") (Utilities|Enum|LiteralenumBPE_EnamyAIState "NewEnumerator1"))
  (AI|Components|Blackboard|SetValueasObject _blackboard (Utilities|Name|MakeLiteralName "TargetActror") 0)
  (AI|ClearFocus)
  (bind _asbp_enemy_base (Utilities|Casting|CastToBP_EnemyBase (Pawn|GetControlledPawn)))
  (Default|SetIsRunning _asbp_enemy_base true))

(fn StartStrolling
  (bind _blackboard (Variables|Default|GetBlackboard))
  (AI|Components|Blackboard|SetValueasObject _blackboard (Utilities|Name|MakeLiteralName "TargetActror") 0)
  (AI|Components|Blackboard|SetValueasEnum _blackboard (Utilities|Name|MakeLiteralName "AIState") (Utilities|Enum|LiteralenumBPE_EnamyAIState "NewEnumerator0"))
  (AI|ClearFocus)
  (bind _asbp_enemy_base (Utilities|Casting|CastToBP_EnemyBase (Pawn|GetControlledPawn)))
  (Default|SetIsRunning _asbp_enemy_base false))