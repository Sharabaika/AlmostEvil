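; Base enemy character that provides shared death, melee attack and movement speed events.
; Death turns the mesh into a physics ragdoll, disables capsule collision and stops the AI controller's brain logic.
; Melee damage hits the AI controller's focus actor if it is within attack range, while a separate attack flag serves animations only.
; Walk speed starts at strolling in construction and switches between running and strolling on request.
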(event Custom|DeathEvent
  (Physics|SetSimulatePhysics (Variables|Character|GetMesh) true)
  (Collision|SetCollisionEnabled (Variables|Collision|GetCapsuleComponent) "NoCollision"))

(event Custom|StartAttack
  (params (isAttacking :type Boolean))
  (Variables|Default|SetisAttacking isAttacking))

(event Custom|TryDealDamageInMele
  (bind _self self)
  (bind _returnvalue (AI|GetAIController _self))
  (bind _returnvalue_2 (Class|AIController|GetFocusActor _returnvalue))
  (Utilities|IsValid _returnvalue
    (:Is%20Valid
      (if (and (Utilities|IsValid _returnvalue_2) (< (Math|Vector|Distance(Vector) (Transformation|GetActorLocation _returnvalue_2) (Transformation|GetActorLocation)) (Variables|Default|GetMaxAttackDist)))
        (Game|Damage|ApplyDamage _returnvalue_2 (Variables|Default|GetAttackDamage) 0 0)))))

(event Custom|SetIsRunning
  (params (IsRunning :type Boolean))
  (Variables|/Script/Engine.CharacterMovementComponent|SetMaxWalkSpeed (Variables|Character|GetCharacterMovement) (select IsRunning (Variables|Default|GetMaxRunningSpeed) (Variables|Default|GetMaxStrollingSpeed))))

(event EventDeath
  (bind _self self)
  (bind _returnvalue (AI|GetAIController _self))
  (CallFunction|DeathEvent)
  (Utilities|IsValid _returnvalue
    (:Is%20Valid
      (AI|Logic|StopLogic (Variables|/Script/AIModule.AIController|GetBrainComponent _returnvalue) "Death"))))

(fn ConstructionScript
  (bind _charactermovement (Variables|Character|GetCharacterMovement))
  (Utilities|IsValid _charactermovement
    (:Is%20Valid
      (Variables|/Script/Engine.CharacterMovementComponent|SetMaxWalkSpeed _charactermovement (Variables|Default|GetMaxStrollingSpeed)))))