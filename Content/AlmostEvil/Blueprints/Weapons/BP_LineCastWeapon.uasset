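; BP_LineCastWeapon is a weapon Blueprint that adds a red laser sight, firing effects and optional noise reporting to its parent's shot behavior.
; While aiming, Tick line-traces from the muzzle on Visibility and feeds the hit distance to the laser, with a fixed length on a miss.
; When not aiming, it zeroes the beam length rather than deactivating it.
; OnShot calls the parent, then can report a noise event; PlayShootingEffects handles muzzle flash and sound.
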(event EventOnStartAiming
  (Variables|Default|SetisAiming true)
  (Components|Activation|Activate (Variables|Default|GetLaserSight) false))

(event EventOnStopAiming
  (Variables|Default|SetisAiming false))

(event EventTick
  (params (DeltaSeconds :type Float%20%28single-precision%29))
  (bind _muzzlelocation (Variables|Default|GetMuzzleLocation))
  (bind _returnvalue (Transformation|GetWorldLocation _muzzlelocation))
  (if (Variables|Default|GetisAiming)
    (bind (_outhit _returnvalue_2) (Collision|LineTraceByChannel _returnvalue (+ _returnvalue (* (Math|Vector|GetForwardVector _muzzlelocation) (Variables|Default|GetMaxDistance))) "TraceTypeQuery1" false 0 "None"))
    (Effects|Components|ParticleSystem|SetVectorParameter (Variables|Default|GetLaserSight) "LaserEnd" (select _returnvalue_2 (Math|Vector|MakeVector (.distance _outhit) 0.0 0.0) "1500.000000, 0, 0"))
    (else
      (Effects|Components|ParticleSystem|SetVectorParameter (Variables|Default|GetLaserSight) "LaserEnd" "0, 0, 0"))))

(event EventBeginPlay
  (Effects|Components|ParticleSystem|SetColorParameter (Variables|Default|GetLaserSight) "BeamColor" "(R=1.000000,G=0.000000,B=0.007180,A=1.000000)"))

(event EventPlayShootingEffects
  (Effects|SpawnEmitterAttached (Variables|Default|GetMuzzleFlash) (Variables|Default|GetMuzzleLocation) "None")
  (Audio|PlaySoundatLocation (Variables|Default|GetFIreSound) (Transformation|GetWorldLocation (Variables|Default|GetMuzzleLocation)) "0, 0, 0" 1.0 1.0 0.0 0 0 0))

(event EventOnShot
  (|CallParentFunction)
  (if (Variables|Default|GetNoiseOnFire)
    (Class|AISenseHearing|ReportNoiseEvent (Transformation|GetActorLocation) (Variables|Default|GetNoise) 0 0.0 "Noise")))

(fn ConstructionScript)