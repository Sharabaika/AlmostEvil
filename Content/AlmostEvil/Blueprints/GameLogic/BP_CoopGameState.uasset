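; Co-op game state that tracks present characters and level quest progress, broadcasting changes through event dispatchers.
; Characters are added uniquely or rebuilt from a supplied list, with additions and switches announced to listeners.
; UpdateLevelState advances the replicated Tasks struct, announced on replication by OnRep, and has the game mode complete the level when the state equals the task count.
; A completion event shows the HUD's final menu and records a win achievement on success.
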(event Custom|AddCharacter
  (params (NewCharacter :type BP%20Third%20Person%20Character%20Object%20Reference%20%28by%20ref%29))
  (bind _presentcharacters (Variables|Default|GetPresentCharacters))
  (bind _returnvalue (Utilities|Array|AddUnique _presentcharacters NewCharacter))
  (if (Utilities|Array|IsValidIndex _presentcharacters _returnvalue)
    (CallFunction|OnCharacterAdded (Variables|Default|GetPresentCharacters))))

(event Custom|OnCharacterSwitched
  (Default|CallOnCharacterSwitchedDP))

(event Custom|OnLevelComplete_Multicast
  (params (Success :type Boolean))
  (bind _returnvalue (Game|GetPlayerController 0))
  (bind _asplayer_hud (Utilities|Casting|CastToPlayerHUD (HUD|GetHUD (Game|GetPlayerController 0))))
  (Default|ShowFinalMenu _asplayer_hud Success)
  (if Success
    (|CacheAchievements _returnvalue
      (:OnSuccess
        (|WriteAchievementProgress _returnvalue "ACH_WIN_ONE_GAME" 1.0)))))

(event Custom|OnCharacterAdded
  (params (PresentCharacters :type Array%20of%20BP%20Third%20Person%20Character%20Object%20References))
  (Default|CallOnCharacterAddedDP PresentCharacters))

(event Custom|ResetCharacters
  (params (NewParam :type Array%20of%20BP%20Third%20Person%20Character%20Object%20References))
  (Utilities|Array|Clear (Variables|Default|GetPresentCharacters))
  (for _array_element NewParam
    (CallFunction|AddCharacter _array_element))
  (CallFunction|OnCharacterAdded (Variables|Default|GetPresentCharacters)))

(fn ConstructionScript)

(fn UpdateLevelState
  (params (NewLevelState :type Integer))
  (Utilities|Struct|SetmembersinS_LevelQuest (Variables|Default|GetTasks) NewLevelState)
  (Default|CallOnLevelStateUpdatedDP (Utilities|Array|Get(acopy) (.tasks (Variables|Default|GetTasks)) NewLevelState))
  (if (== NewLevelState (Utilities|Array|Length (.tasks (Variables|Default|GetTasks))))
    (bind _asbp_coop_game_mode (Utilities|Casting|CastToBP_CoopGameMode (Game|GetGameMode)))
    (Default|CompleteLevel _asbp_coop_game_mode true)))

(fn OnRepTasks
  (bind _tasks (Variables|Default|GetTasks))
  (Default|CallOnLevelStateUpdatedDP (Utilities|Array|Get(acopy) (.tasks _tasks) (.state _tasks))))