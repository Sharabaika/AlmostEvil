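; Lobby game mode that manages players joining, leaving and being kicked, and opens the selected level.
; Joining players register with BP_LobbyGameState, which is cached lazily, and the local first player controller is flagged as host.
; Joins, exits, kicks and ready events re-check the game state's start condition and broadcast the result.
; BeginPlay fills the available levels from a DataTable, and MyGameInstance loads the chosen one.
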(event Custom|KickPlayer
  (params (Player :type Player%20State%20Object%20Reference))
  (bind _asbp_lobby_player_controller (Utilities|Casting|CastToBP_LobbyPlayerController (Components|GetOwner Player)))
  (Default|LeaveLobby _asbp_lobby_player_controller)
  (Default|CallUpdatePlayers (Variables|Default|GetLobbyGameState))
  (CallFunction|UpdateCanStartGame))

(event Custom|OnAnyPlayerReady
  (params (ready :type Boolean))
  (CallFunction|UpdateCanStartGame))

(event Custom|UpdateCanStartGame
  (bind _can (Default|GetCanStartGame (Variables|Default|GetLobbyGameState)))
  (Default|CallOnCanStartGame _can))

(event Custom|OpenSelectedLevel
  (bind _lobbygamestate (Variables|Default|GetLobbyGameState))
  (bind _asmy_game_instance (Utilities|Casting|CastToMyGameInstance (Game|GetGameInstance)))
  (Default|LoadLevel _asmy_game_instance (Utilities|Array|Get(acopy) (Variables|/Game/AlmostEvil/Blueprints/Menuing/Lobby/BP_LobbyGameState.BP_LobbyGameState_C|GetAvailableLevels _lobbygamestate) (Variables|/Game/AlmostEvil/Blueprints/Menuing/Lobby/BP_LobbyGameState.BP_LobbyGameState_C|GetCurrentLevelIndex _lobbygamestate))))

(event Custom|SetLevels
  (bind _outrownames (DataTable|GetDataTableRowNames (Variables|Default|GetLevels)))
  (for _array_element _outrownames
    (bind _returnvalue (Utilities|GetDataTableRow (Variables|Default|GetLevels) _array_element)
      (:then
        (Utilities|Array|AddUnique (Variables|/Game/AlmostEvil/Blueprints/Menuing/Lobby/BP_LobbyGameState.BP_LobbyGameState_C|GetAvailableLevels (Variables|Default|GetLobbyGameState)) _returnvalue)))))

(event EventOnLogout
  (params (ExitingController :type Controller%20Object%20Reference))
  (bind _asbp_lobby_player_controller (Utilities|Casting|CastToBP_LobbyPlayerController ExitingController))
  (Utilities|Array|RemoveItem (Variables|Default|GetPlayers) _asbp_lobby_player_controller)
  (Utilities|Array|RemoveItem (Variables|/Game/AlmostEvil/Blueprints/Menuing/Lobby/BP_LobbyGameState.BP_LobbyGameState_C|GetPlayers (Variables|Default|GetLobbyGameState)) (.AsBP%20Lobby%20Player%20State (Utilities|Casting|CastToBP_LobbyPlayerState (Variables|/Script/Engine.Controller|GetPlayerState _asbp_lobby_player_controller))))
  (Default|CallUpdatePlayers (Variables|Default|GetLobbyGameState))
  (CallFunction|UpdateCanStartGame))

(event EventBeginPlay
  (CallFunction|SetLevels))

(event EventHandleStartingNewPlayer
  (params (NewPlayer :type Player%20Controller%20Object%20Reference))
  (bind _asbp_lobby_player_controller (Utilities|Casting|CastToBP_LobbyPlayerController NewPlayer))
  (CallFunction|AddPlayer _asbp_lobby_player_controller))

(fn ConstructionScript)

(fn AddPlayer
  (params (Player :type BP%20Lobby%20Player%20Controller%20Object%20Reference%20%28by%20ref%29))
  (LocalVariables|SetNewPlayerState (.AsBP%20Lobby%20Player%20State (Utilities|Casting|CastToBP_LobbyPlayerState (Variables|/Script/Engine.Controller|GetPlayerState Player))))
  (Utilities|Array|AddUnique (Variables|Default|GetPlayers) Player)
  (Variables|Default|GetLobbyGameState
    (:then
      _)
    (:else
      (bind _asbp_lobby_game_state (Utilities|Casting|CastToBP_LobbyGameState (Game|GetGameState)))
      (bind _output_get (Variables|Default|SetLobbyGameState _asbp_lobby_game_state))))
  (Default|AddPlayer _output_get (LocalVariables|GetNewPlayerState))
  (Variables|/Game/AlmostEvil/Blueprints/Menuing/Lobby/BP_LobbyPlayerState.BP_LobbyPlayerState_C|SetisHost (LocalVariables|GetNewPlayerState) (== Player (Game|GetPlayerController 0)))
  (EventDispatchers|BindEventtoOnPlayerReady (LocalVariables|GetNewPlayerState) (EventDispatchers|CreateEvent :!event Custom|OnAnyPlayerReady))
  (CallFunction|UpdateCanStartGame))