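; Co-op game mode that sets up joining players, lets them switch between characters and signals level success or failure.
; Each new player takes a color from a spare pool and possesses a character spawned at an unused PlayerStart, which is then registered in BP_CoopGameState.
; Switching cycles that character list to the next one not player-controlled.
; The level fails when no character is alive, and logout resets the list from characters in the world.
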(event Custom|CompleteLevel
  (params (Success :type Boolean))
  (Default|OnLevelCompleteMulticast (Variables|Default|GetCoopGameState) Success))

(event EventBeginPlay
  (bind _asbp_coop_game_state (Utilities|Casting|CastToBP_CoopGameState (Game|GetGameState)))
  (Variables|Default|SetCoopGameState _asbp_coop_game_state))

(event EventHandleStartingNewPlayer
  (params (NewPlayer :type Player%20Controller%20Object%20Reference))
  (Players|SetPlayrColor NewPlayer)
  (bind _newcharacter (Spawning|SpawnPlayerCharacter NewPlayer))
  ;[1 1 1] NEEDED ONLY FOR SINGLE PLAYER  TESTING
  (Utilities|IsValid (Variables|Default|GetCoopGameState)
    (:Is%20Valid
      _)
    (:Is%20Not%20Valid
      (bind _asbp_coop_game_state (Utilities|Casting|CastToBP_CoopGameState (Game|GetGameState)))
      (Variables|Default|SetCoopGameState _asbp_coop_game_state)))
  (Default|AddCharacter (Variables|Default|GetCoopGameState) _newcharacter))

(event EventOnLogout
  (params (ExitingController :type Controller%20Object%20Reference))
  (bind _outactors (Actor|GetAllActorsOfClass "/Game/AlmostEvil/Blueprints/Characters/BP_ThirdPersonCharacter.BP_ThirdPersonCharacter_C"))
  (Default|ResetCharacters (Variables|Default|GetCoopGameState) _outactors))

(fn ConstructionScript)

(fn ChooseSpawnLocation
  (params (Player :type Player%20Controller%20Object%20Reference))
  (if (Variables|Spawning|GetbSpawnsAreFound)
    _
    (else
      (bind _outactors (Actor|GetAllActorsOfClass "/Script/Engine.PlayerStart"))
      (Variables|Spawning|SetAvailableStarts _outactors)
      (Variables|Spawning|SetbSpawnsAreFound true)))
  (Utilities|IsValid (Utilities|Array|Get(acopy) (Variables|Spawning|GetAvailableStarts) (Utilities|Array|LastIndex (Variables|Spawning|GetAvailableStarts)))
    (:Is%20Valid
      (LocalVariables|SetFoundStart (Transformation|GetActorTransform (Utilities|Array|Get(acopy) (Variables|Spawning|GetAvailableStarts) (Utilities|Array|LastIndex (Variables|Spawning|GetAvailableStarts)))))
      (Utilities|Array|RemoveIndex (Variables|Spawning|GetAvailableStarts) (Utilities|Array|LastIndex (Variables|Spawning|GetAvailableStarts))))
    (:Is%20Not%20Valid
      (LocalVariables|SetFoundStart (Math|Transform|MakeTransform "0, 0, 0" "0, 0, 0" "1,1,1"))))
  (return (LocalVariables|GetFoundStart)))

(fn SpawnPlayerCharacter
  (params (Player :type Player%20Controller%20Object%20Reference))
  (bind _spawnpoint (Spawning|ChooseSpawnLocation Player))
  (bind _returnvalue (Game|SpawnActorfromClass "/Game/AlmostEvil/Blueprints/Characters/BP_ThirdPersonCharacter.BP_ThirdPersonCharacter_C" _spawnpoint "Undefined" Player 0))
  (Pawn|Possess Player _returnvalue)
  (return _returnvalue))

(fn TrySwitchActiveCharacterforPlayer
  (params (Player :type Player%20Controller%20Object%20Reference))
  (bind _coopgamestate (Variables|Default|GetCoopGameState))
  (bind _presentcharacters (Variables|/Game/AlmostEvil/Blueprints/GameLogic/BP_CoopGameState.BP_CoopGameState_C|GetPresentCharacters _coopgamestate))
  ;[1 1 1] find controlled character index
  (bind (_array_element _array_index) (Utilities|Array|ForEachLoopwithBreak (Variables|/Game/AlmostEvil/Blueprints/GameLogic/BP_CoopGameState.BP_CoopGameState_C|GetPresentCharacters (Variables|Default|GetCoopGameState)) :!label _label)
    (:LoopBody
      (if (== (Pawn|GetController _array_element) Player)
        (LocalVariables|SetCurrentCharacterIndex _array_index)
        (goto _label Break)))
    (:Completed
      ;[1 1 1] find following spare character
      (if (<= (+ (LocalVariables|GetCurrentCharacterIndex) 1) (Utilities|Array|LastIndex _presentcharacters))
        (LocalVariables|Seti (+ (LocalVariables|GetCurrentCharacterIndex) 1))
        (else
          (LocalVariables|Seti 0)))
      (while (!= (LocalVariables|Geti) (LocalVariables|GetCurrentCharacterIndex))
        (if (Pawn|IsPlayerControlled (Utilities|Array|Get(acopy) _presentcharacters (LocalVariables|Geti)))
          (if (<= (+ (LocalVariables|Geti) 1) (Utilities|Array|LastIndex _presentcharacters))
            (LocalVariables|Seti (+ (LocalVariables|Geti) 1))
            (else
              (LocalVariables|Seti 0)))
          (else
            ;[1 1 1] spaghetti
            (Pawn|Possess Player (Utilities|Array|Get(acopy) _presentcharacters (LocalVariables|Geti)))
            (Default|OnCharacterSwitched (Variables|Default|GetCoopGameState)) ; mb its better to call from playerController OnPossess
            (return)))))))

(fn SetPlayrColor
  (params (Player :type Player%20Controller%20Object%20Reference))
  (bind _spareplayercolors (Variables|Default|GetSparePlayerColors))
  (bind _asbp_coop_player_controller (Utilities|Casting|CastToBP_CoopPlayerController Player))
  (Utilities|IsValid (Variables|/Game/AlmostEvil/Blueprints/GameLogic/BP_CoopPlayerController.BP_CoopPlayerController_C|GetCoopPlayerState _asbp_coop_player_controller)
    (:Is%20Valid
      _)
    (:Is%20Not%20Valid
      ;[1 1 1] single player
      (bind _asbp_coop_player_state (Utilities|Casting|CastToBP_CoopPlayerState (Variables|/Script/Engine.Controller|GetPlayerState _asbp_coop_player_controller)))
      (Variables|/Game/AlmostEvil/Blueprints/GameLogic/BP_CoopPlayerController.BP_CoopPlayerController_C|SetCoopPlayerState _asbp_coop_player_controller _asbp_coop_player_state)))
  (if (Utilities|Array|IsValidIndex _spareplayercolors)
    (Variables|/Game/AlmostEvil/Blueprints/GameLogic/BP_CoopPlayerState.BP_CoopPlayerState_C|SetPlayerColor (Variables|/Game/AlmostEvil/Blueprints/GameLogic/BP_CoopPlayerController.BP_CoopPlayerController_C|GetCoopPlayerState _asbp_coop_player_controller) (Utilities|Array|Get(acopy) _spareplayercolors))
    (Utilities|Array|RemoveIndex _spareplayercolors)))

(fn CheckGameState
  (for _array_element (Variables|/Game/AlmostEvil/Blueprints/GameLogic/BP_CoopGameState.BP_CoopGameState_C|GetPresentCharacters (Variables|Default|GetCoopGameState))
    (if (Variables|/Script/AlmostEvil.ThirdPersonCharacter|GetIsAlive _array_element)
      (return)))
  (CallFunction|CompleteLevel false))